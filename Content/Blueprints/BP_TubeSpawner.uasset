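; BP_TubeSpawner builds a rolling chain of random tube segments along the X axis, keeping a buffer of groups.
; BeginPlay fills the buffer; each group gets randomly rolled TubeClass pieces plus an end BP_NextBox holding a spawner reference.
; PushBuffer spawns the next group, then PopBuffer destroys the oldest.
; Spawned actors are tagged with their group index, so removal works by tag lookup.
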(event Custom|SpawnGroup
  (params (GroupIndexOffset :type Integer))
  (bind _returnvalue (Transformation|GetActorLocation))
  (bind _groupcount (Variables|Default|GetGroupCount))
  (Variables|Default|SetCurrentOffset GroupIndexOffset)
  (for _index (range 0 _groupcount)
    (if (== _index _groupcount)
      (bind _returnvalue_2 (Game|SpawnActorfromClass "/Game/Sch/BP_NextBox.BP_NextBox_C" (Math|Transform|MakeTransform (Math|Vector|MakeVector (+ (.x _returnvalue) (Math|Conversions|ToFloat(Integer) (* _index 68300)) (Math|Conversions|ToFloat(Integer) (* (Variables|Default|GetCurrentOffset) (* _groupcount 68300)))) (.y _returnvalue) (.z _returnvalue)) (Math|Rotator|MakeRotator (Utilities|Select :Index (Math|Random|RandomIntegerinRange 0 3) :Option%200 0.0 :Option%201 9e+01 :Option%202 1.8e+02 :Option%203 2.7e+02) 0.0 0.0)) "AlwaysSpawn" 0 self 0))
      (Variables|Default|SetNextBox _returnvalue_2)
      (Utilities|Array|Add (Variables|/Script/Engine.Actor|GetTags _returnvalue_2) (Utilities|String|StringToName (Utilities|String|ToString(Integer) (Variables|Default|GetCurrentOffset))))
      (else
        (bind _returnvalue_3 (Game|SpawnActorfromClass (.OutItem (Utilities|Array|Random (Variables|Default|GetTubeClass))) (Math|Transform|MakeTransform (Math|Vector|MakeVector (+ (.x _returnvalue) (Math|Conversions|ToFloat(Integer) (* _index 68300)) (Math|Conversions|ToFloat(Integer) (* (Variables|Default|GetCurrentOffset) (* _groupcount 68300)))) (.y _returnvalue) (.z _returnvalue)) (Math|Rotator|MakeRotator (Utilities|Select :Index (Math|Random|RandomIntegerinRange 0 3) :Option%200 0.0 :Option%201 9e+01 :Option%202 1.8e+02 :Option%203 2.7e+02) 0.0 0.0)) "Undefined" 0 0))
        (Utilities|Array|Add (Variables|/Script/Engine.Actor|GetTags _returnvalue_3) (Utilities|String|StringToName (Utilities|String|ToString(Integer) (Variables|Default|GetCurrentOffset))))))))

(event Custom|PushBuffer
  (bind _currentoffset (Variables|Default|GetCurrentOffset))
  (bind _returnvalue (+ _currentoffset 1))
  (Utilities|Array|Add (Variables|Default|GetBuffer) _returnvalue)
  (CallFunction|SpawnGroup _returnvalue)
  (CallFunction|PopBuffer))

(event Custom|PopBuffer
  (bind _buffer (Variables|Default|GetBuffer))
  (bind _outactors (Actor|GetAllActorsOfClasswithTag "/Script/Engine.Actor" (Utilities|String|StringToName (Utilities|String|ToString(Integer) (Utilities|Array|Get(acopy) _buffer)))))
  (for _array_element _outactors
    (Actor|DestroyActor _array_element))
  (Utilities|Array|RemoveIndex _buffer))

(event EventBeginPlay
  (for _index (range 0 (Variables|Default|GetBufferSize))
    (CallFunction|SpawnGroup _index)
    (Utilities|Array|Add (Variables|Default|GetBuffer) _index)))

(event Collision|EventActorBeginOverlap
  (params (OtherActor :type Actor%20Object%20Reference)))

(event EventTick
  (params (DeltaSeconds :type Float%20%28single-precision%29)))

(fn ConstructionScript)
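; Tube actor with two pieces that travel back and forth and a damageable part, Cube2.
; A Timeline lerps Cube and Cube17 along a long path, with a FlipFlop alternating reverse and play.
; AnyDamage adds to Dura and destroys Cube2 past a threshold, while Tick steadily decays Dura.
; Dura shifts Cube2's emissive color from cyan to red through a dynamic material created in the Construction Script.
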(event EventBeginPlay
  (|CallParentFunction)
  (bind _新建轨道_0 (Timeline|时间轴_0 Play)
    (:Update
      (Transformation|SetRelativeLocation (Variables|Default|GetCube) (Math|Vector|Lerp(Vector) "0.000000,11.148010,0.000000" "68300.000000,11.148010,545.000000" _新建轨道_0) false false))
    (:Finished
      (Utilities|FlowControl|FlipFlop
        (:A
          (Timeline|时间轴_0 Reverse))
        (:B
          (Timeline|时间轴_0 Play))))))

(event Collision|EventActorBeginOverlap
  (params (OtherActor :type Actor%20Object%20Reference))
  (|CallParentFunction OtherActor) ; 此节点被禁用，将不会被调用。\n从引脚连出引线来编译功能。
)

(event EventTick
  (params (DeltaSeconds :type Float%20%28single-precision%29))
  (|CallParentFunction DeltaSeconds)
  (Variables|Default|SetDura (Math|Float|Clamp(Float) (+ -0.05 (Variables|Default|GetDura)) 0.0 5.0))
  (bind _cube2 (Variables|Default|GetCube2)
    (:then
      (Rendering|Material|SetVectorParameterValueonMaterials _cube2 "Emissive color 01" (Math|Vector|Lerp(Vector) "0.560000,2.958483,4.000000" "5.000000, 0, 0" (Math|Float|MapRangeClamped (Variables|Default|GetDura) 0.0 5.0 0.0 1.0))))
    (:else)))

(event Game|Damage|EventAnyDamage
  (params (Damage :type Float%20%28single-precision%29) (DamageType :type Damage%20Type%20Object%20Reference) (InstigatedBy :type Controller%20Object%20Reference) (DamageCauser :type Actor%20Object%20Reference))
  (Variables|Default|SetDura (+ Damage (Variables|Default|GetDura)))
  (Math|Float|CompareFloat (+ Damage (Variables|Default|GetDura)) 5.0
    (:>
      (Components|DestroyComponent (Variables|Default|GetCube2) :!label _label))
    (:==
      (goto _label))
    (:<
      (bind _cube2 (Variables|Default|GetCube2)
        (:then
          (Rendering|Material|SetVectorParameterValueonMaterials _cube2 "Emissive color 01" (Math|Vector|Lerp(Vector) "0.560000,2.958483,4.000000" "5.000000, 0, 0" (Math|Float|MapRangeClamped (Variables|Default|GetDura) 0.0 5.0 0.0 1.0))))
        (:else)))))

(fn ConstructionScript
  (bind _cube2 (Variables|Default|GetCube2))
  (|CallParentFunction)
  (bind _returnvalue (Rendering|Material|CreateDynamicMaterialInstance (Rendering|Material|GetMaterial _cube2 0) "None" "None" :!class /Script/Engine.KismetMaterialLibrary))
  (Rendering|Material|SetMaterial _cube2 0 _returnvalue))
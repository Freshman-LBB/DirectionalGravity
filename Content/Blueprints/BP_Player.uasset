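; Player pawn that constantly moves forward, strafes on the MoveRight axis and falls along a switchable gravity axis.
; Tick applies both gravity and movement as swept local offsets, with only gravity scaled by delta time.
; J sets gravity to +Y, while L takes it from the Arrow's forward vector and derives a new actor roll from it.
; Other movement, look and overlap events are empty.
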(event EventBeginPlay
  (Components|Movement|SetUpdatedComponent (Variables|Default|GetFloatingPawnMovement) (Variables|Default|GetSphere)))

(event Collision|EventActorBeginOverlap
  (params (OtherActor :type Actor%20Object%20Reference)))

(event EventTick
  (params (DeltaSeconds :type Float%20%28single-precision%29))
  (Transformation|AddActorLocalOffset (* (Variables|Default|GetGravityAxis) (* DeltaSeconds 9.8e+02)) true false)
  (Transformation|AddActorLocalOffset (Math|Vector|MakeVector 5.0 (* (Variables|Default|GetRightInput) 6.0) 0.0) true false))

(event Input|AxisEvents|InputAxisMoveForward
  (params (AxisValue :type Float%20%28single-precision%29)))

(event Input|AxisEvents|InputAxisMoveRight
  (params (AxisValue :type Float%20%28single-precision%29))
  (Variables|Default|SetRightInput AxisValue))

(event Input|AxisEvents|InputAxisTurn
  (params (AxisValue :type Float%20%28single-precision%29)))

(event Input|AxisEvents|InputAxisLookUp
  (params (AxisValue :type Float%20%28single-precision%29)))

(event Input|KeyboardEvents|J
  (params (Key :type Key%20Structure :default "None"))
  (:Pressed
    (Variables|Default|SetGravityAxis "0,1.000000, 0")))

(event Input|KeyboardEvents|L
  (params (Key :type Key%20Structure :default "None"))
  (:Pressed
    (bind _output_get (Variables|Default|SetGravityAxis (Math|Vector|GetForwardVector (Variables|Default|GetArrow))))
    (Transformation|SetActorRotation (Math|Rotator|MakeRotator (.roll (Math|Rotator|MakeRotfromY _output_get)) 0.0 0.0))))

(fn ConstructionScript)
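; BP_TubeE is an actor whose Cube component slides up and down endlessly along its local Z axis.
; On BeginPlay, a timeline drives a vector lerp that sets the cube's relative location between low and high endpoints, without sweep.
; Each time the timeline finishes, a FlipFlop alternates between Reverse and Play, producing a continuous ping-pong motion.
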(event EventBeginPlay
  (|CallParentFunction)
  (bind _新建轨道_0 (Timeline|时间轴_0 Play)
    (:Update
      (Transformation|SetRelativeLocation (Variables|Default|GetCube) (Math|Vector|Lerp(Vector) "1000.000000, 0,-545.000000" "1000.000000, 0,545.000000" _新建轨道_0) false false))
    (:Finished
      (Utilities|FlowControl|FlipFlop
        (:A
          (Timeline|时间轴_0 Reverse))
        (:B
          (Timeline|时间轴_0 Play))))))

(event Collision|EventActorBeginOverlap
  (params (OtherActor :type Actor%20Object%20Reference))
  (|CallParentFunction OtherActor) ; 此节点被禁用，将不会被调用。\n从引脚连出引线来编译功能。
)

(event EventTick
  (params (DeltaSeconds :type Float%20%28single-precision%29))
  (|CallParentFunction DeltaSeconds) ; 此节点被禁用，将不会被调用。\n从引脚连出引线来编译功能。
)

(fn ConstructionScript
  (|CallParentFunction))
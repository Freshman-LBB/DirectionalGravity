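; First-person auto-runner character that shifts gravity on key presses while grounded, with step, jump and landing sounds.
; J and L rotate gravity a quarter turn either way; I and K chain two turns for a flip.
; Each shift destroys all gravity volumes and spawns a long BP_GravityVolumeBox at the character.
; Tick drives forward movement and accumulates stalled and airborne timers, either of which triggers the game-over widget and removes gravity.
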(event Custom|SpawnGravity
  (params (LocalDirection :type Vector) (Force :type Float%20%28single-precision%29))
  (Game|SpawnActorfromClass "/Game/DirectionalGravity/Blueprints/SceneObjects/BP_GravityVolumeBox.BP_GravityVolumeBox_C" (Math|Transform|MakeTransform (Transformation|GetActorLocation) "0, 0, 0" "999.000000,20.000000,20.000000") "Undefined" 0 LocalDirection Force true 0))

(event Custom|RemoveAllGravity
  (bind _outactors (Actor|GetAllActorsOfClass "/Game/DirectionalGravity/Blueprints/GravityLogic/BP_GravityVolumeBase.BP_GravityVolumeBase_C"))
  (for _array_element _outactors
    (Actor|DestroyActor _array_element)))

(event Custom|OnStep
  (if (and (Variables|Default|GetbStart) (Variables|Default|GetIsOnGround))
    (Audio|PlaySound2D "/Game/DirectionalGravity/Meshes/-hc1eto3s6odgs0n5.-hc1eto3s6odgs0n5" 2.0 1.0 0.0 0 0)))

(event Custom|Replay
  (Audio|Components|Audio|Play (stale EventBeginPlay _returnvalue) 0.0))

(event EventBeginPlay
  (Utilities|Time|SetTimerbyEvent (delegate Custom|OnStep) 0.5 true)
  (bind _returnvalue (AddComponent|AddAudioComponent false))
  (EventDispatchers|BindEventtoOnAudioFinished _returnvalue (delegate Custom|Replay)))

(event Collision|EventActorBeginOverlap
  (params (OtherActor :type Actor%20Object%20Reference)))

(event EventTick
  (params (DeltaSeconds :type Float%20%28single-precision%29))
  (bind _returnvalue (Game|GetPlayerController 0))
  (|CallParentFunction DeltaSeconds)
  (Utilities|FlowControl|Sequence
    (:then_0
      (if (Variables|Default|GetbStart)
        (Variables|Default|SetForwardDeltaMove 1.0)
        (Utilities|FlowControl|Sequence
          (:then_0
            (if (< (Math|Vector|VectorLength (Transformation|GetVelocity)) 1e+02)
              (Variables|Default|SetBlock (Math|Float|Clamp(Float) (+ (Variables|Default|GetBlock) (* (Utilities|Time|GetWorldDeltaSeconds) (/ 1.0 2.0)))))
              (else
                (Variables|Default|SetBlock (Math|Float|Clamp(Float) (- (Variables|Default|GetBlock) (* (Utilities|Time|GetWorldDeltaSeconds) (/ 1.0 3.0))))))))
          (:then_1
            (if (Variables|Default|GetIsOnGround)
              (Variables|Default|SetAir (Math|Float|Clamp(Float) (- (Variables|Default|GetAir) (* (Utilities|Time|GetWorldDeltaSeconds) (/ 1.0 0.001)))))
              (else
                (Variables|Default|SetAir (Math|Float|Clamp(Float) (+ (Variables|Default|GetAir) (* (Utilities|Time|GetWorldDeltaSeconds) (/ 1.0 2.0))))))))
          (:then_2
            (if (or (Math|Float|NearlyEqual(Float) (Variables|Default|GetBlock) 1.0 1e-06) (Math|Float|NearlyEqual(Float) (Variables|Default|GetAir) 1.0 1e-06))
              (Utilities|FlowControl|DoOnce false
                (:Completed
                  (bind _returnvalue_2 (UserInterface|CreateWidget "/Game/Sch/UMG_GameOver.UMG_GameOver_C"))
                  (UserInterface|Viewport|AddtoViewport _returnvalue_2 0)
                  (Input|SetInputModeUIOnly _returnvalue 0 "DoNotLock")
                  (Variables|/Script/Engine.PlayerController|SetbShowMouseCursor _returnvalue true)
                  (CallFunction|RemoveAllGravity)))))
          (:then_3
            (if (Variables|Default|GetIsOnGround)
              (if (Variables|Default|GetCanPlayLandSound)
                (Audio|PlaySound2D "/Game/Sch/-3lne1cckoddy6i92.-3lne1cckoddy6i92" 1.0 1.0 0.0 0 0)
                (Variables|Default|SetCanPlayLandSound false))
              (else
                (Variables|Default|SetCanPlayLandSound true)))))))))

(event Input|KeyboardEvents|J
  (params (Key :type Key%20Structure :default "None"))
  (:Pressed
    (if (and (Variables|Default|GetbStart) (Variables|Default|GetIsOnGround))
      (CallFunction|RemoveAllGravity)
      (Variables|Default|SetDirection (Math|Vector|MakeVector 0.0 (.Z (Math|Vector|BreakVector (Variables|Default|GetDirection))) (* (.Y (Math|Vector|BreakVector (Variables|Default|GetDirection))) -1.0)))
      (CallFunction|SpawnGravity (Variables|Default|GetDirection) 4e+03)
      (Audio|PlaySound2D "/Game/Sch/-rxrf096iete4zcea.-rxrf096iete4zcea" 1.0 1.0 0.0 0 0))))

(event Input|KeyboardEvents|K
  (params (Key :type Key%20Structure :default "None"))
  (:Pressed
    (if (and (Variables|Default|GetbStart) (Variables|Default|GetIsOnGround))
      (CallFunction|RemoveAllGravity)
      (Variables|Default|SetDirection (Math|Vector|MakeVector 0.0 (* (.Z (Math|Vector|BreakVector (Variables|Default|GetDirection))) -1.0) (.Y (Math|Vector|BreakVector (Variables|Default|GetDirection)))))
      (Utilities|FlowControl|Sequence
        (:then_0
          (CallFunction|SpawnGravity (Variables|Default|GetDirection) 4e+03)
          (Utilities|FlowControl|Delay 0.1)
          (CallFunction|RemoveAllGravity)
          (Variables|Default|SetDirection (Math|Vector|MakeVector 0.0 (* (.Z (Math|Vector|BreakVector (Variables|Default|GetDirection))) -1.0) (.Y (Math|Vector|BreakVector (Variables|Default|GetDirection)))))
          (CallFunction|SpawnGravity (Variables|Default|GetDirection) 1.5e+03))
        (:then_1
          (Audio|PlaySound2D "/Game/Sch/-rxrf096iete4zcea.-rxrf096iete4zcea" 1.0 1.0 0.0 0 0))))))

(event Input|KeyboardEvents|L
  (params (Key :type Key%20Structure :default "None"))
  (:Pressed
    (if (and (Variables|Default|GetbStart) (Variables|Default|GetIsOnGround))
      (CallFunction|RemoveAllGravity)
      (Variables|Default|SetDirection (Math|Vector|MakeVector 0.0 (* (.Z (Math|Vector|BreakVector (Variables|Default|GetDirection))) -1.0) (.Y (Math|Vector|BreakVector (Variables|Default|GetDirection)))))
      (CallFunction|SpawnGravity (Variables|Default|GetDirection) 4e+03)
      (Audio|PlaySound2D "/Game/Sch/-rxrf096iete4zcea.-rxrf096iete4zcea" 1.0 1.0 0.0 0 0))))

(event Input|KeyboardEvents|I
  (params (Key :type Key%20Structure :default "None"))
  (:Pressed
    (if (and (Variables|Default|GetbStart) (Variables|Default|GetIsOnGround))
      (CallFunction|RemoveAllGravity)
      (Variables|Default|SetDirection (Math|Vector|MakeVector 0.0 (* (.Z (Math|Vector|BreakVector (Variables|Default|GetDirection))) -1.0) (.Y (Math|Vector|BreakVector (Variables|Default|GetDirection)))))
      (Utilities|FlowControl|Sequence
        (:then_0
          (CallFunction|SpawnGravity (Variables|Default|GetDirection) 4e+03)
          (Utilities|FlowControl|Delay 0.1)
          (CallFunction|RemoveAllGravity)
          (Variables|Default|SetDirection (Math|Vector|MakeVector 0.0 (* (.Z (Math|Vector|BreakVector (Variables|Default|GetDirection))) -1.0) (.Y (Math|Vector|BreakVector (Variables|Default|GetDirection)))))
          (CallFunction|SpawnGravity (Variables|Default|GetDirection) 1.5e+03))
        (:then_1
          (Audio|PlaySound2D "/Game/Sch/-rxrf096iete4zcea.-rxrf096iete4zcea" 1.0 1.0 0.0 0 0))))))

(fn ConstructionScript
  (|CallParentFunction))